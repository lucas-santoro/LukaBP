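; Dialogue component for the Mouse character, defining its branching conversation with placeholder test lines.
; Overrides Dialogue, calls the parent, then switches on DialogueTreeIndex, chaining AddDialogue nodes by pass-through state and chosen option.
; Branches end by closing the conversation after advancing the tree index, removing some progress or clearing it.
; Tree 1 is the finished state, showing one of two random lines with a single Continue option.
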(fn `Dialogue`
  (`parent.Dialogue`)
  (switch `int` (`self.DialogueTreeIndex`)
    (:`0`
      (bind (_state _optionindex) (`self.AddDialogue` "Mouse" "Test text" (`|MakeArray` "Option 1" "Option 2" :!type "Text")))
      (switch `/Game/Dialogue_Sys/Enum_DialogueState` _state
        (:`NewEnumerator0`
          (switch `int` _optionindex
            (:`0`
              (bind (_state_2 _optionindex_2) (`self.AddDialogue` "Mouse" "You have choosed option 1" (`|MakeArray` "Option 1" "Option 2" :!type "Text")))
              (switch `/Game/Dialogue_Sys/Enum_DialogueState` _state_2
                (:`NewEnumerator0`
                  (switch `int` _optionindex_2
                    (:`0`
                      (bind _state_3 (`self.AddDialogue` "Mouse" "You have choosed option 2" (`|MakeArray` "Option 1" "Option 2" "Option 3" "Option 4" :!type "Text")))
                      (switch `/Game/Dialogue_Sys/Enum_DialogueState` _state_3
                        (:`NewEnumerator0`
                          (`self.SetDialogueTreeIndex` 1)
                          (`self.CloseConversation`))))
                    (:`1`
                      (bind _state_4 (`self.AddDialogue` "Mouse" "AAAAAAAAAAAA" (`|MakeArray` "Option 1" "Option 2" "Option 3" "Option 4" :!type "Text")))
                      (switch `/Game/Dialogue_Sys/Enum_DialogueState` _state_4
                        (:`NewEnumerator0`
                          (`self.RemoveDialogueProgress` 2)
                          (`self.CloseConversation`))))))))
            (:`1`
              (bind _state_5 (`self.AddDialogue` "Mouse" "You have choosed option 2" (`|MakeArray` "Option 1" "Option 2" "Option 3" "Option 4" :!type "Text")))
              (switch `/Game/Dialogue_Sys/Enum_DialogueState` _state_5
                (:`NewEnumerator0`
                  (`self.ClearDialogueProgress`)
                  (`self.CloseConversation`))))))))
    (:`1`
      (bind _state_6 (`self.AddDialogue` "Mouse" (select `int` (`KismetMathLibrary.RandomIntegerInRange` 0 1) :`0` "Finished dialogue random option 1" :`1` "TextFinished dialogue random option 2" :!type "Text") (`|MakeArray` "Continue" :!type "Text")))
      (switch `/Game/Dialogue_Sys/Enum_DialogueState` _state_6
        (:`NewEnumerator0`
          (`self.ClearDialogueProgress`)
          (`self.CloseConversation`))))))